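; Gameplay player controller that gives the player an in-game chat widget, created on BeginPlay.
; GetChatMessage relays text with the stored sender name through GamePlayGM's list of all player controllers, calling UpdateChat on each to refresh its chat window.
; The Chut input toggles the mouse cursor via FlipFlop.
; LoadGame loads the player settings save slot but leaves the result unused.
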(event `self.ReceiveBeginPlay`
  ;[1 1 1] Присвоение имени игроку
  (`self.CreatChutWindow`))

(event `CreatChutWindow`
  ;[1 1 1] Создание игрового чата и добавление его во вьюпорт
  (bind _returnvalue (`|CreateWidget` "/Game/UI/WB_GamePlayChat.WB_GamePlayChat_C"))
  (bind _output_get (set `self.GamePlayChatWB` _returnvalue))
  (if (`KismetSystemLibrary.IsValid` _output_get)
    (`UserWidget.AddToViewport` _output_get 0)))

(event `UpdateName`
  (params (Name :type Text))
  ;[1 1 1] Присовение имени игроку
  (set `self.SenderName` Name))

(event `GetChatMessage`
  (params (TextToSend :type Text))
  ;[1 1 1] Comment
  (set `self.SenderText` TextToSend)
  (bind _asgame_play_gm (cast `/Game/Blueprints/GameplayGM/GamePlayGM` (`GameplayStatics.GetGameMode`)))
  (for _array_element (`/Game/Blueprints/GameplayGM/GamePlayGM.AllPlayerControllers` _asgame_play_gm)
    (bind _asgame_play_pc (cast `/Game/Blueprints/GameplayGM/GamePlayPC` _array_element))
    (`self.UpdateChat` _asgame_play_pc (`self.SenderName`) (`self.SenderText`))))

(event `UpdateChat`
  (params (SenderName :type Text) (SenderText :type Text))
  ;[1 1 1] Обновление чата у клиента
  (`/Game/UI/WB_ChatWindow.UpdateChatWindow` (`/Game/UI/WB_GamePlayChat.GamePlayChat` (`self.GamePlayChatWB`)) SenderName SenderText))

(event `InputAction|Chut`
  (params (Key :type "Key Structure"))
  ;[1 1 1] Подключиться отключиться от чата
  (:`Pressed`
    (`/Engine/EditorBlueprintResources/StandardMacros.FlipFlop`
      (:`A`
        (set `self.bShowMouseCursor` true))
      (:`B`
        (set `self.bShowMouseCursor` false)))))

(fn `LoadGame`
  (`GameplayStatics.LoadGameFromSlot` (`self.PlayerSettingSave`)))

(fn `UserConstructionScript`)